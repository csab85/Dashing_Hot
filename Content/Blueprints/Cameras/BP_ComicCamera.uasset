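; Comic-page camera that pans between panel positions and hands the view back to the gameplay camera on arrival.
; BeginPlay gathers scene captures, comic frames and the gameplay camera.
; While Tick interpolates toward the active position, the previous panel's capture takes a snapshot and the active one captures live.
; On arrival, live capture stops, the gameplay camera gets that panel's distance limits, and frame-visibility toggling is left unconnected.
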(event `self.ReceiveBeginPlay`
  ;[1 1 1] Get scene capturers and frames
  (bind _outactors (`GameplayStatics.GetAllActorsOfClass` "/Script/Engine.SceneCapture2D"))
  (set `self.SceneCapurers` _outactors)
  (bind _outactors_2 (`GameplayStatics.GetAllActorsOfClass` "/Game/Blueprints/UI/Comics/BP_ComicFrame.BP_ComicFrame_C"))
  (set `self.Frames` _outactors_2)
  (bind _returnvalue (`GameplayStatics.GetActorOfClass` "/Game/Blueprints/Cameras/BP_GameplayCamera.BP_GameplayCamera_C"))
  (set `self.Gameplay Camera` _returnvalue))

(event `self.ReceiveTick`
  (params (DeltaSeconds :type "Float (single-precision)"))
  (bind _gameplay_camera (`self.Gameplay Camera`))
  (bind _gameplay_camera_2 (`self.Gameplay Camera`))
  (bind (_output_x _output_y) (`KismetMathLibrary.BreakVector2D` (`|GetArrayItem` (`self.MaxDistances`) (`self.ActivePosition`))))
  (if (== (`self.K2_GetActorLocation`) (`|GetArrayItem` (`self.Positions`) (`self.ActivePosition`)))
    ;[1 1 1] Deactivate scene capture
    (if (`self.Changing`)
      (set `SceneCaptureComponent.bCaptureEveryFrame` false (`SceneCapture2D.CaptureComponent2D` (`|GetArrayItem` (`self.SceneCapurers`) (`self.ActivePosition`))))
      (set `self.Changing` false)
      ;[1 1 1] Set new max distances
      (set `/Game/Blueprints/Cameras/BP_GameplayCamera.Max X Distance` _output_x _gameplay_camera)
      (set `/Game/Blueprints/Cameras/BP_GameplayCamera.Max Y Distance` _output_y _gameplay_camera)
      ;[1 1 1] Change to gameplay camera
      (`/Game/Blueprints/Cameras/BP_GameplayCamera.UpdateActiveLocation` _gameplay_camera_2)
      (`PlayerController.SetViewTargetWithBlend` (`GameplayStatics.GetPlayerController` 0) _gameplay_camera_2 0.0 "VTBlend_Linear" 0.0 false))
    (else
      ;[1 1 1] Capture screen and activate scene capture
      (if (not (`self.Changing`))
        (`SceneCaptureComponent2D.CaptureScene` (`SceneCapture2D.CaptureComponent2D` (`|GetArrayItem` (`self.SceneCapurers`) (`self.LastPosition`))))
        (set `SceneCaptureComponent.bCaptureEveryFrame` true (`SceneCapture2D.CaptureComponent2D` (`|GetArrayItem` (`self.SceneCapurers`) (`self.ActivePosition`))))
        (set `self.Changing` true)
        ;[1 1 1] change to comic camera
        (`PlayerController.SetViewTargetWithBlend` (`GameplayStatics.GetPlayerController` 0) self 0.0 "VTBlend_Linear" 0.0 false))
      ;[1 1 1] Move towards correct location
      (`self.K2_SetActorTransform` (`KismetMathLibrary.MakeTransform` (`KismetMathLibrary.VInterpTo` (`self.K2_GetActorLocation`) (`|GetArrayItem` (`self.Positions`) (`self.ActivePosition`)) 0.3 0.5) (`self.K2_GetActorRotation`))))))

(fn `ChangeSquare`
  (`SceneCaptureComponent2D.CaptureScene` (`SceneCapture2D.CaptureComponent2D` (`|GetArrayItem` (`self.SceneCapurers`) (`self.LastPosition`))))
  (set `SceneCaptureComponent.bCaptureEveryFrame` true (`SceneCapture2D.CaptureComponent2D` (`|GetArrayItem` (`self.SceneCapurers`) (`self.ActivePosition`))))
  (set `self.Changing` true))

(fn `UserConstructionScript`)