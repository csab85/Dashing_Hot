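; BP_GameplayCamera is a gameplay camera that sits at a stored position for the active area and leans slightly toward the player.
; BeginPlay finds BP_Player, then each Tick offsets the area position by a tenth of the player's distance from the camera in X and Y.
; Each axis updates only within its maximum distance, and Z stays unchanged.
; The Transition function is an empty stub.
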(event `self.ReceiveBeginPlay`
  (bind _returnvalue (`GameplayStatics.GetActorOfClass` "/Game/Blueprints/Player/BP_Player.BP_Player_C"))
  (set `self.Player` _returnvalue))

(event `self.ReceiveTick`
  (params (DeltaSeconds :type "Float (single-precision)"))
  (bind (_returnvalue_x _returnvalue_y _returnvalue_z) (`KismetMathLibrary.BreakVector` (`self.K2_GetActorLocation`)))
  (bind _returnvalue_x_2 (`KismetMathLibrary.BreakVector` (`self.K2_GetActorLocation`)))
  (bind (_returnvalue_x_3 _returnvalue_y_2) (`KismetMathLibrary.BreakVector` (`self.K2_GetActorLocation`)))
  (bind _returnvalue_x_4 (`KismetMathLibrary.BreakVector` (`self.K2_GetActorLocation` (`self.Player`))))
  (bind (_returnvalue_x_5 _returnvalue_y_3) (`KismetMathLibrary.BreakVector` (`self.K2_GetActorLocation` (`self.Player`))))
  (bind (_output_x _output_y) (`KismetMathLibrary.BreakVector` (`|GetArrayItem` (`self.Positions`) (`self.ActiveArea`))))
  (bind _output_x_2 (`KismetMathLibrary.BreakVector` (`|GetArrayItem` (`self.Positions`) (`self.ActiveArea`))))
  (bind _returnvalue (- _returnvalue_y_3 _returnvalue_y_2))
  (bind _returnvalue_2 (- _returnvalue_x_4 _returnvalue_x_2))
  (`|ExecutionSequence`
    (:`then_0`
      ;[1 1 1] New X
      (if (<= (`KismetMathLibrary.Abs` _returnvalue_2) (`self.Max X Distance`))
        (set `self.X Position` (+ _output_x_2 (* _returnvalue_2 0.1)))))
    (:`then_1`
      ;[1 1 1] New Y
      (if (<= (`KismetMathLibrary.Abs` _returnvalue) (`self.Max Y Distance`))
        (set `self.Y Position` (+ _output_y (* _returnvalue 0.1)))))
    (:`then_2`
      ;[1 1 1] Offset location
      (`self.K2_SetActorLocation` (`KismetMathLibrary.MakeVector` (`self.X Position`) (`self.Y Position`) _returnvalue_z)))))

(fn `Transition`)

(fn `UserConstructionScript`)