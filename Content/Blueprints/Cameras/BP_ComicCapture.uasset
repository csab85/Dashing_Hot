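; BP_ComicCapture is a 2D scene capture actor that mirrors the view position of the gameplay camera.
; On BeginPlay it finds and stores the BP_GameplayCamera in the level.
; Each tick, while its capture component is set to capture every frame, it copies that camera's actor transform and prints its own name for debugging.
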(event `self.ReceiveBeginPlay`
  (bind _returnvalue (`GameplayStatics.GetActorOfClass` "/Game/Blueprints/Cameras/BP_GameplayCamera.BP_GameplayCamera_C"))
  (set `self.Gameplay Camera` _returnvalue))

(event `self.ReceiveTick`
  (params (DeltaSeconds :type "Float (single-precision)"))
  (if (`SceneCaptureComponent.bCaptureEveryFrame` (`self.CaptureComponent2D`))
    (`KismetSystemLibrary.PrintString` (`KismetSystemLibrary.GetDisplayName` self))
    (`self.K2_SetActorTransform` (`self.GetTransform` (`self.Gameplay Camera`)))))

(fn `UserConstructionScript`)