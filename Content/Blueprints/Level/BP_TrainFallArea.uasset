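; BP_TrainFallArea is a level area that hurls gameplay characters along negative world X, apparently to mimic falling off a moving train.
; Begin and end overlap events add and remove each GameplayCharacter in an AffectedChars list.
; Every tick it overwrites the X velocity of each listed character's movement component with a large fixed value, leaving Y and Z untouched.
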(event `self.ReceiveActorBeginOverlap`
  (params (OtherActor :type "Actor Object Reference"))
  (bind _asgameplay_character (cast `GameplayCharacter` OtherActor))
  (`KismetArrayLibrary.Array_Add` (`self.Affected Chars`) _asgameplay_character))

(event `self.ReceiveActorEndOverlap`
  (params (OtherActor :type "Actor Object Reference"))
  (bind _asgameplay_character (cast `GameplayCharacter` OtherActor))
  (`KismetArrayLibrary.Array_RemoveItem` (`self.Affected Chars`) _asgameplay_character))

(event `self.ReceiveTick`
  (params (DeltaSeconds :type "Float (single-precision)"))
  (for _array_element (`self.Affected Chars`)
    (bind _charactermovement (`Character.CharacterMovement` _array_element))
    (bind (_velocity_x _velocity_y _velocity_z) (`KismetMathLibrary.BreakVector` (`MovementComponent.Velocity` _charactermovement)))
    (set `MovementComponent.Velocity` (`KismetMathLibrary.MakeVector` -10000.0 _velocity_y _velocity_z) _charactermovement)))

(fn `UserConstructionScript`)