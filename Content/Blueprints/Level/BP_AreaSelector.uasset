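; BP_AreaSelector is a level actor that switches the active area for the gameplay and comic cameras when the player overlaps it.
; On BeginPlay it caches references to BP_GameplayCamera and BP_ComicCamera.
; On overlap with BP_Player, it saves the comic camera's active position as its last position, then assigns its Area value to both cameras.
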(event `self.ReceiveBeginPlay`
  (bind _returnvalue (`GameplayStatics.GetActorOfClass` "/Game/Blueprints/Cameras/BP_GameplayCamera.BP_GameplayCamera_C"))
  (set `self.GameplayCamera` _returnvalue)
  (bind _returnvalue_2 (`GameplayStatics.GetActorOfClass` "/Game/Blueprints/Cameras/BP_ComicCamera.BP_ComicCamera_C"))
  (set `self.ComicCamera` _returnvalue_2))

(event `self.ReceiveActorBeginOverlap`
  (params (OtherActor :type "Actor Object Reference"))
  (bind _area (`self.Area`))
  (bind _comiccamera (`self.ComicCamera`))
  (cast `/Game/Blueprints/Player/BP_Player` OtherActor)
  (set `/Game/Blueprints/Cameras/BP_ComicCamera.LastPosition` (`/Game/Blueprints/Cameras/BP_ComicCamera.ActivePosition` _comiccamera) _comiccamera)
  (set `/Game/Blueprints/Cameras/BP_GameplayCamera.ActiveArea` _area (`self.GameplayCamera`))
  (set `/Game/Blueprints/Cameras/BP_ComicCamera.ActivePosition` _area (`self.ComicCamera`)))

(fn `UserConstructionScript`)