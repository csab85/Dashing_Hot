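; BP_NextLevel is a level exit that advances the player to the next level once every enemy is defeated.
; It counts Enemy actors on BeginPlay into EnemiesAlive, which is not decremented in this file, and Tick swaps the mesh material when the count reaches zero.
; Player overlap with the mesh then opens the entry following the current level's name in the Levels array.
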(event `self.ReceiveBeginPlay`
  (bind _outactors (`GameplayStatics.GetAllActorsOfClass` "/Script/Dashing_Hot.Enemy"))
  (set `self.EnemiesAlive` (`KismetArrayLibrary.Array_Length` _outactors)))

(event `self.ReceiveTick`
  (params (DeltaSeconds :type "Float (single-precision)"))
  (if (not (> (`self.EnemiesAlive`) 0))
    (`PrimitiveComponent.SetMaterial` (`self.StaticMeshComponent`) 0 "/Engine/MapTemplates/Materials/BasicAsset03.BasicAsset03")))

(event `self.StaticMeshComponent.OnComponentBeginOverlap`
  (params (OverlappedComponent :type "PrimitiveComponent Object Reference") (OtherActor :type "Actor Object Reference") (OtherComp :type "PrimitiveComponent Object Reference") (OtherBodyIndex :type Integer) (bFromSweep :type Boolean) (SweepResult :type "HitResult Structure (by ref)"))
  (bind _levels (`self.Levels`))
  (cast `/Game/Blueprints/Player/BP_Player` OtherActor)
  (if (<= (`self.EnemiesAlive`) 0)
    (bind _returnvalue (`GameplayStatics.GetCurrentLevelName` true))
    (`GameplayStatics.OpenLevel` (`|GetArrayItem` _levels (+ (`KismetArrayLibrary.Array_Find` _levels (`KismetStringLibrary.Conv_StringToName` _returnvalue)) 1)))))

(fn `UserConstructionScript`)