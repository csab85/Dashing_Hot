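; BP_BaseEnemy is an enemy Blueprint, apparently a base class, that links enemy state to its AI Blackboard.
; On BeginPlay it caches the AI controller's Blackboard and the BP_Player actor, then calls SetStates with a starting state.
; SetStates writes the State enum to the Blackboard's "State" key and sets the Dashing flag only for one specific shooter state.
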(event `self.ReceiveBeginPlay`
  (`|ExecutionSequence`
    (:`then_0`
      ;[1 1 1] Get Blackboard Reference
      (set `self.Blackboard` (`AIBlueprintHelperLibrary.GetBlackboard` (`AIBlueprintHelperLibrary.GetAIController` self))))
    (:`then_1`
      ;[1 1 1] Get reference to player
      (bind _returnvalue (`GameplayStatics.GetActorOfClass` "/Game/Blueprints/Player/BP_Player.BP_Player_C"))
      (set `self.player` _returnvalue))
    (:`then_2`
      ;[1 1 1] Set starting state
      (`self.SetStates` "NewEnumerator10"))))

(fn `SetStates`
  (params (State :type "/Game/Blueprints/AI/EnemyShooter/ShooterStates Enum" :default "NewEnumerator0"))
  (bind _output_get (set `local.State` "NewEnumerator0"))
  (`BlackboardComponent.SetValueAsEnum` (`self.Blackboard`) "State" _output_get)
  (if (== (`local.State`) (`KismetSystemLibrary.MakeLiteralByte` (enumliteral `/Game/Blueprints/AI/EnemyShooter/ShooterStates` "NewEnumerator3")))
    (set `self.bDashing` true)
    (else
      (set `self.bDashing` false))))

(fn `UserConstructionScript`)