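; Enemy shooter projectile that damages and stuns gameplay characters on hit.
; A hit on an unstunned character subtracts health, applies an impulse from its negated, scaled velocity, then spawns a laser-hit Niagara effect and destroys itself.
; Other hits and lifetime expiry share a path that first calls the projectile-impact dispatcher, then runs the same effect and cleanup.
; Hits on already stunned characters are ignored.
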(event `self.ReceiveBeginPlay`
  (`KismetSystemLibrary.Delay` (`self.Lifetime`))
  (`self.OnProjectileImpact` (stale `self.ReceiveHit` Other) (stale `self.ReceiveHit` Hit) :!label _label)
  (`NiagaraFunctionLibrary.SpawnSystemAtLocation` "/Game/Art/NE_System/Enemy/NS_LaserHit.NS_LaserHit" (`.Location` (`GameplayStatics.BreakHitResult` (stale `self.ReceiveHit` Hit))) :!label _label_2)
  (`self.K2_DestroyActor`))

(event `self.ReceiveHit`
  (params (MyComp :type "PrimitiveComponent Object Reference") (Other :type "Actor Object Reference") (OtherComp :type "PrimitiveComponent Object Reference") (bSelfMoved :type Boolean) (HitLocation :type "Vector Structure") (HitNormal :type "Vector Structure") (NormalImpulse :type "Vector Structure") (Hit :type "HitResult Structure (by ref)"))
  (bind (_returnvalue_x _returnvalue_y) (`KismetMathLibrary.BreakVector` (* (`self.GetVelocity`) -250.0)))
  (bind _asgameplay_character (cast `GameplayCharacter` Other)
    (:`then`
      (if (not (`GameplayCharacter.bStunned` _asgameplay_character))
        (set `GameplayCharacter.Health` (- (`GameplayCharacter.Health` _asgameplay_character) (`self.damage`)) _asgameplay_character)
        (`CharacterMovementComponent.AddImpulse` (`Character.CharacterMovement` _asgameplay_character) (`KismetMathLibrary.MakeVector` _returnvalue_x _returnvalue_y) false)
        (set `GameplayCharacter.bStunned` true _asgameplay_character)
        (goto _label_2)))
    (:`CastFailed`
      (goto _label))))

(fn `UserConstructionScript`)