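; Blocker enemy that takes damage and knockback from player dashes and is destroyed shortly after health runs out.
; Capsule hits subtract player damage and, if the player can hit, switch it to OnAir for a timed knockback before Stunned.
; Tick applies knockback velocity while airborne and updates the health bar widget.
; SetStates always writes 0 to the Blackboard State key, and LookAtLocation is an empty stub.
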(event `self.ReceiveBeginPlay`
  (`|ExecutionSequence`
    (:`then_0`
      ;[1 1 1] Get Blackboard Reference
      (set `self.Blackboard` (`AIBlueprintHelperLibrary.GetBlackboard` (`AIBlueprintHelperLibrary.GetAIController` self))))
    (:`then_1`
      ;[1 1 1] Get reference to player
      (bind _returnvalue (`GameplayStatics.GetActorOfClass` "/Game/Blueprints/Player/BP_Player.BP_Player_C"))
      (set `self.player` _returnvalue))
    (:`then_2`
      ;[1 1 1] Set starting state
      (`self.SetStates` "NewEnumerator0"))))

(event `self.ReceiveTick`
  (params (DeltaSeconds :type "Float (single-precision)"))
  (`|ExecutionSequence`
    (:`then_0`
      ;[1 1 1] Update projectile spawnpoint location
      (set `self.ProjectileSpawn` (`SceneComponent.K2_GetComponentLocation` (`self.ProjectileSpawnpoint`))))
    (:`then_1`
      (switch `/Game/Blueprints/AI/EnemyBlocker/BlockerStates` (`self.State`)
        (:`NewEnumerator4`
          (set `MovementComponent.Velocity` (* (`self.knockbackDirection`) 100 (`/Game/Blueprints/Player/BP_Player.FinalDashPushForce` (`self.player`))) (`self.CharacterMovement`)))))
    (:`then_2`
      (bind _aswb_enemy (cast `/Game/Blueprints/UI/WB_Enemy` (`WidgetComponent.GetWidget` (`self.UI`))))
      (`ProgressBar.SetPercent` (`/Game/Blueprints/UI/WB_Enemy.HealthBar` _aswb_enemy) (/ (`self.Health`) (`self.MaxHealth`))))
    (:`then_3`
      ;[1 1 1] Destroy if health lower than 0
      (if (<= (`self.Health`) 0.0)
        (`KismetSystemLibrary.Delay` 0.5)
        (`self.K2_DestroyActor`)))
    (:`then_4`
      ;[1 1 1] Look at player
      (`self.LookAtLocation` (`self.K2_GetActorLocation` (`self.player`))))))

(event `self.CapsuleComponent.OnComponentHit`
  (params (HitComponent :type "PrimitiveComponent Object Reference") (OtherActor :type "Actor Object Reference") (OtherComp :type "PrimitiveComponent Object Reference") (NormalImpulse :type "Vector Structure") (Hit :type "HitResult Structure (by ref)"))
  ;[1 0.1569 0.1961] Hit on Capsule Component
  (`|ExecutionSequence`
    (:`then_0`
      (bind _asbp_player (cast `/Game/Blueprints/Player/BP_Player` OtherActor))
      ;[0.3882 1 0.3333] Lower health
      (set `self.Health` (- (`self.Health`) (`/Game/Blueprints/Player/BP_Player.FinalDamage` _asbp_player)))
      ;[0.3882 1 0.3333] Update knockback direction
      (`NavMovementComponent.StopActiveMovement` (`self.CharacterMovement`))
      (if (`/Game/Blueprints/Player/BP_Player.CanHit` _asbp_player)
        (set `self.knockbackDirection` (`NewPlayer.DashDirection` (`self.player`)))
        ;[0.3882 1 0.3333] Control knockback duration
        (`self.SetStates` "NewEnumerator4")
        (`KismetSystemLibrary.Delay` (`self.KnockbackDuration`))
        (`self.SetStates` "NewEnumerator5")))))

(event `self.ProximityDetector.OnComponentBeginOverlap`
  (params (OverlappedComponent :type "PrimitiveComponent Object Reference") (OtherActor :type "Actor Object Reference") (OtherComp :type "PrimitiveComponent Object Reference") (OtherBodyIndex :type Integer) (bFromSweep :type Boolean) (SweepResult :type "HitResult Structure (by ref)"))
  ;[0.3882 1 0.3333] Activate if player closer
  (cast `/Game/Blueprints/Player/BP_Player` OtherActor)
  (set `self.RepositionRadius` (`self.RepositionNormalRadius`))
  (`self.SetStates` "NewEnumerator0"))

(fn `LookAtLocation`
  (params (TargetLocation :type "Vector Structure")))

(fn `SetStates`
  (params (State :type "/Game/Blueprints/AI/EnemyBlocker/BlockerStates Enum" :default "NewEnumerator0"))
  (set `self.State` State)
  (`BlackboardComponent.SetValueAsEnum` (`self.Blackboard`) "State" 0)
  (if (== (`local.State`) (`KismetSystemLibrary.MakeLiteralByte` (enumliteral `/Game/Blueprints/AI/EnemyBlocker/BlockerStates` "NewEnumerator0")))
    (set `self.bDashing` true)
    (else
      (set `self.bDashing` false))))

(fn `UserConstructionScript`)