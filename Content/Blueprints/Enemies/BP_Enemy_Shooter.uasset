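; BP_Enemy_Shooter is an enemy that gets knocked back when it collides with the player while the player's CanHit is set.
; A capsule hit stores a normalized direction pointing away from the player and raises a Flying flag for KnockbackDuration.
; While Flying, Tick overrides CharacterMovement velocity along that direction, scaled by the player's DashHitForce.
; Despite the name, it contains no shooting logic.
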(event `self.ReceiveBeginPlay`
  (`|ExecutionSequence`
    (:`then_0`
      ;[1 1 1] Get reference to player
      (bind _returnvalue (`GameplayStatics.GetActorOfClass` "/Game/Blueprints/BP_Player.BP_Player_C"))
      (set `self.player` _returnvalue))))

(event `self.ReceiveTick`
  (params (DeltaSeconds :type "Float (single-precision)"))
  (`|ExecutionSequence`
    (:`then_0`
      ;[0.3765 0.6863 1] Add dash force if dashing
      (if (`self.flying`)
        (set `MovementComponent.Velocity` (* (`self.knockbackDirection`) 100 (`NewPlayer.dashHitForce` (`self.player`))) (`self.CharacterMovement`))))))

(event `self.CapsuleComponent.OnComponentHit`
  (params (HitComponent :type "PrimitiveComponent Object Reference") (OtherActor :type "Actor Object Reference") (OtherComp :type "PrimitiveComponent Object Reference") (NormalImpulse :type "Vector Structure") (Hit :type "HitResult Structure (by ref)"))
  ;[1 0.1569 0.1961] Hit on Capsule Component
  (bind _asbp_player (cast `/Game/Blueprints/BP_Player` OtherActor))
  ;[0.3882 1 0.3333] Update knockback direction
  (if (`/Game/Blueprints/BP_Player.bCanHit` _asbp_player)
    (bind _knockbackdirection (`self.GetKnockbackDirection`))
    (set `self.knockbackDirection` _knockbackdirection)
    ;[0.3882 1 0.3333] Control knockback duration
    (set `self.flying` true)
    (`KismetSystemLibrary.Delay` (`self.KnockbackDuration`))
    (set `self.flying` false)))

(fn `GetKnockbackDirection`
  (returns (knockbackDirection :type "Vector Structure"))
  (bind _returnvalue (`MyBlueprintFunctionLibrary.GetVectorToLocation` (`self.K2_GetActorLocation` self) (`self.K2_GetActorLocation` (`self.player`)) true true))
  (return _returnvalue))

(fn `UserConstructionScript`)