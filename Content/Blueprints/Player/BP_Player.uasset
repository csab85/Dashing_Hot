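; Player character with mouse-aimed dash combat: normal, slow-motion double, charged and explosive leap dashes.
; Enhanced Input triggers dashes, gated by state, cooldown or Heat cost, aimed by a cursor trace ignoring comic camera frames.
; Tick drives dash velocity, stun, flame effects and level restart on death.
; StopDashing, called on timeout or collision, scales damage and push by dash time and charge, setting punch flags and adding Heat on enemy hits.
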(event `self.ReceiveBeginPlay`
  (`|ExecutionSequence`
    (:`then_0`
      ;[1 1 1] Set Player Controller
      (set `self.PlayerController` (`GameplayStatics.GetPlayerController` 0)))
    (:`then_1`
      ;[1 1 1] Enable Player Mapping
      (`EnhancedInputSubsystemInterface.AddMappingContext` (pcsubsystem `EnhancedInputLocalPlayerSubsystem` (`self.PlayerController`)) "/Game/Inputs/Player_Mapping.Player_Mapping" 0 (struct)))
    (:`then_2`
      ;[1 1 1] Show Mouse
      (set `PlayerController.bShowMouseCursor` true (`self.PlayerController`)))
    (:`then_3`
      (bind _returnvalue (`GameplayStatics.GetActorOfClass` "/Game/Blueprints/Cameras/BP_ComicCamera.BP_ComicCamera_C"))
      (set `self.Comic Camera` _returnvalue))))

(event `self.ReceiveTick`
  (params (DeltaSeconds :type "Float (single-precision)"))
  (bind _charactermovement (`self.CharacterMovement`))
  (bind _mesh (`self.Mesh`))
  (bind _fire (`self.Fire`))
  (bind (_returnvalue_x _returnvalue_y) (`KismetMathLibrary.BreakVector` (* (`self.dashDirection`) 100 (`self.dashSpeed`) (`self.ChargeMultiplier`))))
  (bind (_velocity_x _velocity_y _velocity_z) (`KismetMathLibrary.BreakVector` (`MovementComponent.Velocity` _charactermovement)))
  (`|ExecutionSequence`
    (:`then_0`
      (if (`self.bDashing`)
        (`|ExecutionSequence`
          (:`then_0`
            (set `MovementComponent.Velocity` (`KismetMathLibrary.MakeVector` _returnvalue_x _returnvalue_y _velocity_z) _charactermovement))
          (:`then_1`
            (set `self.TimeDashing` (+ DeltaSeconds (`self.TimeDashing`))))
          (:`then_2`
            (`PrimitiveComponent.SetCollisionResponseToChannel` (`self.CapsuleComponent`) "ECC_Destructible" "ECR_Ignore")))
        (else
          (`|ExecutionSequence`
            (:`then_1`
              (`PrimitiveComponent.SetCollisionResponseToChannel` (`self.CapsuleComponent`) "ECC_Destructible" "ECR_Block"))))))
    (:`then_1`
      (if (`self.bStunned`)
        (set `self.Charging` false)
        (`KismetSystemLibrary.Delay` (`self.StunDuration`))
        (set `self.bStunned` false)))
    (:`then_2`
      (if (<= (`self.Health`) 0.0)
        (`GameplayStatics.OpenLevel` "Subway_Station")))
    (:`then_3`
      (if (or (`self.bDashing`) (`self.Jumping`))
        (set `self.SecondsToUnfire` (`self.BaseUnfireTime`))
        (`MeshComponent.SetOverlayMaterial` _mesh "/Game/Art/Materials/Vfx/M_OverlayFlame_Inst.M_OverlayFlame_Inst")
        (`ActorComponent.Activate` _fire true)
        (else
          (bind _output_get (set `self.SecondsToUnfire` (- (`self.SecondsToUnfire`) DeltaSeconds)))
          (if (<= _output_get 0.0)
            (`MeshComponent.SetOverlayMaterial` _mesh null)
            (`ActorComponent.Deactivate` _fire)))))))

(event `EnhancedInput|/Game/Inputs/Walk`
  (params (ActionValue :type "Vector2D Structure") (ElapsedSeconds :type "Float (double-precision)") (TriggeredSeconds :type "Float (double-precision)") (InputAction :type "InputAction Object Reference" :default "/Game/Inputs/Walk.Walk"))
  (bind _returnvalue (`KismetMathLibrary.Conv_Vector2DToVector` ActionValue))
  (:`Triggered`
    ;[1 1 1] Check if can walk
    (if (`self.bStunned`)
      _
      (elif (or (`self.Idle`) (`self.Moving`))
        (if (not (`self.bDashing`))
          (`self.AddMovementInput` _returnvalue)
          (`SceneComponent.K2_SetWorldRotation` (`self.Mesh`) (`KismetMathLibrary.MakeRotFromX` _returnvalue) false false)
          (`SceneComponent.K2_AddLocalRotation` (`self.Mesh`) (struct :`Yaw` -90.0) false false)
          (set `self.Moving` true)
          (set `self.Idle` false)))))
  (:`Completed`
    ;[1 1 1] Reset once not walking
    (set `self.Moving` false)
    (if (not (`self.bDashing`))
      (set `self.Idle` true))))

(event `EnhancedInput|/Game/Inputs/Dash`
  (params (ActionValue :type Boolean) (ElapsedSeconds :type "Float (double-precision)") (TriggeredSeconds :type "Float (double-precision)") (InputAction :type "InputAction Object Reference" :default "/Game/Inputs/Dash.Dash"))
  (:`Triggered`
    (bind _canuseskill (`self.CheckIfCanUseSkill` 0.0))
    (if _canuseskill
      (`self.Dash` false))))

(event `EnhancedInput|/Game/Inputs/Double_Dash`
  (params (ActionValue :type Boolean) (ElapsedSeconds :type "Float (double-precision)") (TriggeredSeconds :type "Float (double-precision)") (InputAction :type "InputAction Object Reference" :default "/Game/Inputs/Double_Dash.Double_Dash"))
  (:`Triggered`
    (`self.Double Dash`))
  (:`Ongoing`
    (if (>= ElapsedSeconds (`self.SlowMoStartTime`))
      (bind _can_use_skill (`self.CheckHeatMinimum` (`self.DoubleDashHeatUsage`)))
      (if _can_use_skill
        (`self.Aim Double Dash`)
        (else
          (`GameplayStatics.SetGlobalTimeDilation` 1.0))))))

(event `EnhancedInput|/Game/Inputs/Charge_Dash`
  (params (ActionValue :type Boolean) (ElapsedSeconds :type "Float (double-precision)") (TriggeredSeconds :type "Float (double-precision)") (InputAction :type "InputAction Object Reference" :default "/Game/Inputs/Charge_Dash.Charge_Dash"))
  (:`Ongoing`
    (bind _canuseskill (`self.CheckIfCanUseSkill` (`self.ChargedDashHeatUsage`)))
    (if (or _canuseskill (`self.Charging`))
      (`self.Charge`)))
  (:`Completed`
    (if (`self.Charging`)
      (`self.Discharge`))))

(event `EnhancedInput|/Game/Inputs/Jump_Dash`
  (params (ActionValue :type Boolean) (ElapsedSeconds :type "Float (double-precision)") (TriggeredSeconds :type "Float (double-precision)") (InputAction :type "InputAction Object Reference" :default "/Game/Inputs/Jump_Dash.Jump_Dash"))
  (:`Triggered`
    (bind _canuseskill (`self.CheckIfCanUseSkill` (`self.ExplosiveDashHeatUsage`)))
    (if _canuseskill
      (`self.ExplosiveDash`))))

(event `self.CapsuleComponent.OnComponentHit`
  (params (HitComponent :type "PrimitiveComponent Object Reference") (OtherActor :type "Actor Object Reference") (OtherComp :type "PrimitiveComponent Object Reference") (NormalImpulse :type "Vector Structure") (Hit :type "HitResult Structure (by ref)"))
  ;[1 0.1569 0.1961] Hit on Capsule Component
  (bind _output_get (set `self.Colliding Actor` OtherActor))
  (if (`self.bDashing`)
    (`self.Stop Dashing` true (`KismetMathLibrary.ClassIsChildOf` (`GameplayStatics.GetObjectClass` _output_get) "/Script/Dashing_Hot.Enemy"))))

(event `EnhancedInput|/Game/Inputs/Pause_Game`
  (params (ActionValue :type Boolean) (ElapsedSeconds :type "Float (double-precision)") (TriggeredSeconds :type "Float (double-precision)") (InputAction :type "InputAction Object Reference" :default "/Game/Inputs/Pause_Game.Pause_Game"))
  (:`Triggered`
    (`GameplayStatics.SetGamePaused` true)
    (`WidgetBlueprintLibrary.SetInputMode_UIOnlyEx` (`GameplayStatics.GetPlayerController` 0) null)
    (bind _returnvalue (`|CreateWidget` "/Game/Blueprints/UI/Menu/Pause.Pause_C"))
    (`UserWidget.AddToViewport` _returnvalue 0)
    (set `PlayerController.bShowMouseCursor` true (`GameplayStatics.GetPlayerController` 0))))

(fn `CheckHeatMinimum`
  (params (`Heat Minimum` :type "Float (double-precision)"))
  (returns (`Can Use Skill` :type Boolean))
  (locals (`Can Use` :type Boolean))
  (bind _heat (`self.Heat`))
  (if (>= _heat `Heat Minimum`)
    (set `local.Can Use` true)
    (set `self.Heat` (- _heat `Heat Minimum`))
    (else
      (set `local.Can Use` false)))
  (return (`local.Can Use`)))

(fn `CheckIfCanUseSkill`
  (params (`Heat Minimum` :type "Float (double-precision)"))
  (returns (CanUseSkill :type Boolean))
  (locals (CanUse :type Boolean))
  (bind _can_use_skill (`self.CheckHeatMinimum` `Heat Minimum`))
  (if (and _can_use_skill (or (`self.Idle`) (`self.Moving`)))
    (if (`KismetMathLibrary.BooleanNOR` (`self.bStunned`) (`self.bDashCoolingDown`))
      (set `self.Idle` false)
      (set `self.Moving` false)
      (set `local.CanUse` true)
      (else
        (set `local.CanUse` false :!label _label)))
    (else
      (goto _label)))
  (return (`local.CanUse`)))

(fn `GetAndFaceDashDirection`
  (returns (dashDirection :type "Vector Structure"))
  (locals (`Final X` :type "Float (double-precision)") (`Final Y` :type "Float (double-precision)") (`Final Z` :type "Float (double-precision)"))
  (bind _playercontroller (`self.PlayerController`))
  (bind (_worldlocation _worlddirection) (`PlayerController.DeprojectMousePositionToWorld` _playercontroller))
  ;[1 1 1] Draw line to world poosition
  (bind _outhit (`KismetSystemLibrary.LineTraceSingle` (`PlayerCameraManager.GetCameraLocation` (`PlayerController.PlayerCameraManager` _playercontroller)) (+ _worldlocation (* _worlddirection 1000000.0)) "TraceTypeQuery1" false (`/Game/Blueprints/Cameras/BP_ComicCamera.Frames` (`self.Comic Camera`))))
  (bind _returnvalue (`KismetMathLibrary.Normal` (- (`.Location` (`GameplayStatics.BreakHitResult` _outhit)) (`self.K2_GetActorLocation`))))
  ;[1 1 1] Make player face click direction
  (`SceneComponent.K2_SetWorldRotation` (`self.Mesh`) (`KismetMathLibrary.MakeRotFromX` _returnvalue) false false)
  (`SceneComponent.K2_AddLocalRotation` (`self.Mesh`) (struct :`Yaw` -90.0) false false)
  (return _returnvalue))

(fn `UserConstructionScript`)