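; Anim notify that fires the player's explosive dash blast when its animation reaches the notify.
; It plays the explosion sound and VFX and spawns a large BP_ForceField with radial magnitude at the player.
; A sphere trace for pawns subtracts dash damage directly from each hit enemy's health.
; It also flags those enemies as dashing with a knockback direction away from the player and sets the player's final push force.
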(fn `Received_Notify`
  (params (MeshComp :type "SkeletalMeshComponent Object Reference") (Animation :type "AnimSequenceBase Object Reference") (EventReference :type "AnimNotifyEventReference Structure (by ref)"))
  (returns (ReturnValue :type Boolean))
  (locals (Player :type "/Game/Blueprints/Player/BP_Player Object Reference") (Enemy :type "Enemy Object Reference"))
  (bind _returnvalue (`Actor.K2_GetActorLocation` (`local.Player`)))
  (bind _asbp_player (cast `/Game/Blueprints/Player/BP_Player` (`ActorComponent.GetOwner` MeshComp)))
  ;[1 1 1] Play sfx
  (bind _output_get (set `local.Player` _asbp_player))
  (`GameplayStatics.PlaySoundAtLocation` (`/Game/Blueprints/Player/BP_Player.Explosion SFX` _output_get) (`Actor.K2_GetActorLocation` _output_get) (struct) 1.0 1.0 0.0 null null null null)
  ;[1 1 1] Play VFX
  (`ActorComponent.Activate` (`/Game/Blueprints/Player/BP_Player.Explosion VFX` (`local.Player`)) true)
  (bind _returnvalue_2 (`|SpawnActorFromClass` "/Game/Blueprints/Fields/BP_ForceField.BP_ForceField_C" (`Actor.GetTransform` (`local.Player`)) "AlwaysSpawn" "MultiplyWithRoot" null null))
  (set `/Engine/EditorResources/FieldNodes/FS_MasterField.Radial Magnitude` 2000.0 _returnvalue_2)
  (`Actor.SetActorScale3D` _returnvalue_2 (15.0 15.0 15.0))
  (bind _outhits (`KismetSystemLibrary.SphereTraceMultiForObjects` _returnvalue _returnvalue (`NewPlayer.ExplosiveDashRadius` (`local.Player`)) (`|MakeArray` "ObjectTypeQuery3" :!type "EObjectTypeQuery Enum")))
  (for _array_element _outhits
    (bind (_bblockinghit _binitialoverlap _time _distance _location _impactpoint _normal _impactnormal _physmat _hitactor) (`GameplayStatics.BreakHitResult` _array_element))
    (bind _asenemy (cast `Enemy` _hitactor))
    (`KismetSystemLibrary.PrintString` (`KismetSystemLibrary.GetDisplayName` _hitactor))
    ;[1 1 1] Update health
    (bind _output_get_2 (set `local.Enemy` _asenemy))
    (set `GameplayCharacter.Health` (- (`GameplayCharacter.Health` _output_get_2) (`NewPlayer.ExplosiveDashDamage` (`local.Player`))) _output_get_2)
    ;[1 1 1] Set knackback directiopn
    (set `/Game/Blueprints/Player/BP_Player.FinalDashPushForce` 100.0 (`local.Player`))
    (set `GameplayCharacter.bDashing` true (`local.Enemy`))
    (set `Enemy.KnockbackDirection` (`KismetMathLibrary.Normal` (- (`Actor.K2_GetActorLocation` (`local.Enemy`)) (`Actor.K2_GetActorLocation` (`local.Player`)))) (`local.Enemy`))))