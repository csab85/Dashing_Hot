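; BP_DigitalClock is a scenery Blueprint that displays the current real-world time as a digital clock.
; Every Tick it reads Now() and writes the hour, minute and second into separate Hours, Minutes and Seconds text elements.
; Each value is padded to at least two digits, with seconds converted to a double and formatted without decimals.
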(event `self.ReceiveTick`
  (params (DeltaSeconds :type "Float (single-precision)"))
  (bind _returnvalue (`KismetMathLibrary.Now`))
  (`TextRenderComponent.K2_SetText` (`self.Hours`) (`KismetTextLibrary.Conv_IntToText` (`KismetMathLibrary.GetHour` _returnvalue) false true 2))
  (`TextRenderComponent.K2_SetText` (`self.Minutes`) (`KismetTextLibrary.Conv_IntToText` (`KismetMathLibrary.GetMinute` _returnvalue) false true 2))
  (`TextRenderComponent.K2_SetText` (`self.Seconds`) (`KismetTextLibrary.Conv_DoubleToText` (`KismetMathLibrary.Conv_IntToDouble` (`KismetMathLibrary.GetSecond` _returnvalue)) "HalfToEven" false true 2 324 0 0)))

(fn `UserConstructionScript`)