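; BP_Wall is a scenery wall that bounces and damages Enemy characters that hit it.
; On Hit, it casts the other actor to Enemy and applies an impulse along the wall's forward vector to its CharacterMovement, scaled by speed and BounceForce.
; It then subtracts Health in proportion to the enemy's speed and DamageMultiplier, so faster impacts bounce and hurt more.
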(event `self.ReceiveHit`
  (params (MyComp :type "PrimitiveComponent Object Reference") (Other :type "Actor Object Reference") (OtherComp :type "PrimitiveComponent Object Reference") (bSelfMoved :type Boolean) (HitLocation :type "Vector Structure") (HitNormal :type "Vector Structure") (NormalImpulse :type "Vector Structure") (Hit :type "HitResult Structure (by ref)"))
  (bind _returnvalue (`KismetMathLibrary.VSize` (`MovementComponent.Velocity` (`Character.CharacterMovement` (`self.Enemy`)))))
  (bind _asenemy (cast `Enemy` Other))
  (bind _output_get (set `self.Enemy` _asenemy))
  (`CharacterMovementComponent.AddImpulse` (`Character.CharacterMovement` _output_get) (* (`self.GetActorForwardVector`) _returnvalue (`self.BounceForce`)) false)
  (set `GameplayCharacter.Health` (- (`GameplayCharacter.Health` (`self.Enemy`)) (* (/ _returnvalue 1000.0) (`self.DamageMultiplier`) 0.23)) (`self.Enemy`)))

(fn `UserConstructionScript`)