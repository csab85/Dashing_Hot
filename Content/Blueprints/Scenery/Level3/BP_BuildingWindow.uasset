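; Level 3 scenery actor for a building window that moves repeatedly between two positions.
; Tick waits through a StartTime delay, then plays a Timeline from the start whenever the Moving flag is clear.
; The Timeline's Alpha lerps actor location from InitialPosit to FinalPosit without sweep, and its finish clears Moving so the motion replays.
; StartTime is zeroed while moving, so the delay only offsets the first run.
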(event `self.ReceiveTick`
  (params (DeltaSeconds :type "Float (single-precision)"))
  (`KismetSystemLibrary.Delay` (`self.Start Time`))
  (if (`self.Moving`)
    (set `self.Start Time` 0.0)
    (else
      (bind (_direction _alpha) (`Timeline|Timeline` :!via `PlayFromStart`)
        (:`Update`
          (set `self.Moving` true)
          (`self.K2_SetActorLocation` (`KismetMathLibrary.VLerp` (`self.Initial Posit`) (`self.Final Posit`) _alpha)))
        (:`Finished`
          (set `self.Moving` false))))))

(fn `UserConstructionScript`
  (`parent.UserConstructionScript`))