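; Level 3 elevator actor that detects when no pawns other than the player remain around it and signals the building windows to end their movement cycle.
; While not Stopped, Tick runs through a five-second Delay, then box-traces for pawns, ignoring the player, and prints the hit count.
; With zero hits, it sets LastMovement on every BP_BuildingWindow flagged ShouldMove.
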(event `self.ReceiveTick`
  (params (DeltaSeconds :type "Float (single-precision)"))
  (bind _returnvalue (`self.K2_GetActorLocation`))
  (if (not (`self.Stopped`))
    (`KismetSystemLibrary.Delay` 5.0)
    (bind _returnvalue_2 (`GameplayStatics.GetActorOfClass` "/Game/Blueprints/Player/BP_Player.BP_Player_C"))
    (bind _outhits (`KismetSystemLibrary.BoxTraceMultiForObjects` _returnvalue _returnvalue (1200.0 1000.0 500.0) (struct) (`|MakeArray` "ObjectTypeQuery3" :!type "EObjectTypeQuery Enum") false (`|MakeArray` _returnvalue_2 :!type "Actor Object Reference")))
    (bind _returnvalue_3 (`KismetArrayLibrary.Array_Length` _outhits))
    (`KismetSystemLibrary.PrintString` (`KismetStringLibrary.Conv_IntToString` _returnvalue_3))
    (if (== _returnvalue_3 0)
      (bind _outactors (`GameplayStatics.GetAllActorsOfClass` "/Game/Blueprints/Scenery/Level3/BP_BuildingWindow.BP_BuildingWindow_C"))
      (for _array_element _outactors
        (if (`/Game/Blueprints/Scenery/Level3/BP_BuildingWindow.Should Move` _array_element)
          (set `/Game/Blueprints/Scenery/Level3/BP_BuildingWindow.Last Movement` true _array_element))))))

(fn `UserConstructionScript`)