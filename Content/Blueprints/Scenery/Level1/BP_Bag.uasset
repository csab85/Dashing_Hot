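; BP_Bag is a Level 1 scenery prop built on a Geometry Collection that reacts to dashing characters and projectiles.
; Any overlap releases its constraint and enables gravity; dashes and projectiles also spawn a BP_ForceField scaled by impact velocity.
; That impact damages the overlapping actor if it is an Enemy, with a briefly held actor list filtering duplicates.
; Hits from anything except a non-dashing player disable the hit component's collision.
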(event `self.ReceiveBeginPlay`
  (bind _output_get (set `self.Self Colliders` (`self.K2_GetComponentsByClass` "/Script/Engine.BoxComponent")))
  (for _array_element _output_get
    _))

(event `self.GeometryCollectionComponent.OnComponentBeginOverlap`
  (params (OverlappedComponent :type "PrimitiveComponent Object Reference") (OtherActor :type "Actor Object Reference") (OtherComp :type "PrimitiveComponent Object Reference") (OtherBodyIndex :type Integer) (bFromSweep :type Boolean) (SweepResult :type "HitResult Structure (by ref)"))
  (bind _other_actor (`self.Other Actor`))
  (bind _collidingactors (`self.CollidingActors`))
  (bind _master_field_scale (`self.Master Field Scale`))
  (bind _other_actor_2 (`self.Other Actor`))
  (bind _returnvalue (`KismetMathLibrary.VSize` (`self.GetVelocity` (`self.Other Actor`))))
  (`PrimitiveComponent.SetConstraintMode` (`self.GeometryCollectionComponent`) "None")
  (`PrimitiveComponent.SetConstraintMode` (`self.GeometryCollectionComponent`) "None")
  (`PrimitiveComponent.SetEnableGravity` (`self.GeometryCollectionComponent`) true)
  (set `self.Other Actor` OtherActor)
  ;[1 1 1] Get actor velocity to calculate force and damage
  (set `self.Damage` (/ _returnvalue 1000.0))
  (set `self.ForcePower` (/ _returnvalue 2.25))
  ;[1 1 1] Chechk if dashing character or attack
  (`|ExecutionSequence`
    (:`then_0`
      (bind _asgameplay_character (cast `GameplayCharacter` _other_actor))
      (if (`GameplayCharacter.bDashing` _asgameplay_character)
        ;[1 1 1] Get if actor on collision list (and add if not)
        (if (not (`KismetArrayLibrary.Array_Contains` _collidingactors _other_actor_2)) :!label _label
          (`KismetArrayLibrary.Array_Add` _collidingactors _other_actor_2)
          ;[1 1 1] Reduce health if enemy
          (bind _asenemy (cast `Enemy` (`self.Other Actor`))
            (:`then`
              (set `GameplayCharacter.Health` (- (`GameplayCharacter.Health` _asenemy) (* (`self.DamageMultiplier`) (`self.Damage`) 0.23)) _asenemy))
            (:`CastFailed`
              _))
          ;[1 1 1] Spawn force field
          (bind _returnvalue_2 (`|SpawnActorFromClass` "/Game/Blueprints/Fields/BP_ForceField.BP_ForceField_C" (`KismetMathLibrary.MakeTransform` (`self.K2_GetActorLocation` (`self.Other Actor`)) (struct) (`KismetMathLibrary.MakeVector` _master_field_scale _master_field_scale _master_field_scale)) "AlwaysSpawn" "MultiplyWithRoot" null null))
          (set `/Engine/EditorResources/FieldNodes/FS_MasterField.Radial Magnitude` (`KismetMathLibrary.VSize` (* (`self.ForcePower`) (`self.GetActorScale3D`))) _returnvalue_2)
          ;[1 1 1] Wait then remove firts item from array
          (`KismetSystemLibrary.Delay` 0.05)
          (`KismetArrayLibrary.Array_Remove` (`self.CollidingActors`)))))
    (:`then_1`
      (cast `/Game/Blueprints/Enemies/Shooter/BP_Projectile` _other_actor)
      (goto _label))))

(event `self.ReceiveHit`
  (params (MyComp :type "PrimitiveComponent Object Reference") (Other :type "Actor Object Reference") (OtherComp :type "PrimitiveComponent Object Reference") (bSelfMoved :type Boolean) (HitLocation :type "Vector Structure") (HitNormal :type "Vector Structure") (NormalImpulse :type "Vector Structure") (Hit :type "HitResult Structure (by ref)"))
  (bind _asbp_player (cast `/Game/Blueprints/Player/BP_Player` Other)
    (:`then`
      (if (`GameplayCharacter.bDashing` _asbp_player)
        (`PrimitiveComponent.SetCollisionEnabled` MyComp "NoCollision" :!label _label_2)))
    (:`CastFailed`
      (goto _label_2))))

(fn `UserConstructionScript`)