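; BP_Obstacle is a scenery actor that reacts to dashing or knocked-back characters and projectiles hitting it.
; On CollisionArea overlap, it derives an impact force from the incoming actor's speed.
; Dashing enemies lose health proportional to that force.
; Dashing characters and projectiles both spawn a BP_ForceField at their location, with radial magnitude set from the force and DamageMultiplier.
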(event `self.CollisionArea.OnComponentBeginOverlap`
  (params (OverlappedComponent :type "PrimitiveComponent Object Reference") (OtherActor :type "Actor Object Reference") (OtherComp :type "PrimitiveComponent Object Reference") (OtherBodyIndex :type Integer) (bFromSweep :type Boolean) (SweepResult :type "HitResult Structure (by ref)"))
  ;[1 1 1] Get actor velocity to calculate force
  (set `self.ForcePower` (/ (`KismetMathLibrary.VSize` (`self.GetVelocity` OtherActor)) 6.0))
  (`|ExecutionSequence`
    (:`then_0`
      ;[1 1 1] If gameplay character and dashing (or knockback)
      (bind _asgameplay_character (cast `GameplayCharacter` OtherActor))
      (if (`GameplayCharacter.bDashing` _asgameplay_character)
        ;[1 1 1] Reduce health if enemy
        (bind _asenemy (cast `Enemy` _asgameplay_character)
          (:`then`
            (set `GameplayCharacter.Health` (- (`GameplayCharacter.Health` _asenemy) (/ (`self.ForcePower`) 200.0)) _asenemy))
          (:`CastFailed`
            _))
        ;[1 1 1] Spawn force field
        (bind _returnvalue (`|SpawnActorFromClass` "/Game/Blueprints/Fields/BP_ForceField.BP_ForceField_C" (`KismetMathLibrary.Conv_VectorToTransform` (`self.K2_GetActorLocation` OtherActor)) "AlwaysSpawn" "MultiplyWithRoot" null null :!label _label))
        (set `/Engine/EditorResources/FieldNodes/FS_MasterField.Radial Magnitude` (* (`self.ForcePower`) (`self.DamageMultiplier`)) _returnvalue)))
    (:`then_1`
      ;[1 1 1] If projectile (or any attack type)
      (cast `/Game/Blueprints/Enemies/BP_Projectile` OtherActor)
      (goto _label))))

(fn `UserConstructionScript`)