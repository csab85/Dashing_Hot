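; Player character with Enhanced Input walking and a mouse-aimed dash attack, plus pause menu and level restart on death.
; Dash faces the cursor's screen-space direction, spawns Niagara trail and smoke, then Tick drives velocity and ignores Destructible collision.
; Timeout or capsule hit ends the dash, deriving damage and push force from time dashed before starting cooldown.
; Hitting an Enemy also sets a punching flag.
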(event `self.ReceiveBeginPlay`
  (`|ExecutionSequence`
    (:`then_0`
      ;[1 1 1] Set Player Controller
      (set `self.PlayerController` (`GameplayStatics.GetPlayerController` 0)))
    (:`then_1`
      ;[1 1 1] Enable Player Mapping
      (`EnhancedInputSubsystemInterface.AddMappingContext` (pcsubsystem `EnhancedInputLocalPlayerSubsystem` (`self.PlayerController`)) "/Game/Inputs/Player_Mapping.Player_Mapping" 0 (struct)))
    (:`then_2`
      ;[1 1 1] Show Mouse
      (set `PlayerController.bShowMouseCursor` true (`self.PlayerController`)))))

(event `self.ReceiveTick`
  (params (DeltaSeconds :type "Float (single-precision)"))
  (`|ExecutionSequence`
    (:`then_0`
      (if (`self.bDashing`)
        (`|ExecutionSequence`
          (:`then_0`
            (set `MovementComponent.Velocity` (* (`self.dashDirection`) 100 (`self.dashSpeed`)) (`self.CharacterMovement`)))
          (:`then_1`
            (set `self.TimeDashing` (+ DeltaSeconds (`self.TimeDashing`))))
          (:`then_2`
            (`PrimitiveComponent.SetCollisionResponseToChannel` (`self.CapsuleComponent`) "ECC_Destructible" "ECR_Ignore"))
          (:`then_3`
            (set `self.Moving` false :!label _label)))
        (else
          (`|ExecutionSequence`
            (:`then_0`
              (if (== (`MovementComponent.Velocity` (`self.CharacterMovement`)) (0.0 0.0 0.0))
                (goto _label)
                (else
                  (set `self.Moving` true))))
            (:`then_1`
              (`PrimitiveComponent.SetCollisionResponseToChannel` (`self.CapsuleComponent`) "ECC_Destructible" "ECR_Block"))))))
    (:`then_1`
      (if (<= (`self.Health`) 0.0)
        (`GameplayStatics.OpenLevel` "Subway_Station")))))

(event `EnhancedInput|/Game/Inputs/Player_Walk`
  (params (ActionValue :type "Vector2D Structure") (ElapsedSeconds :type "Float (double-precision)") (TriggeredSeconds :type "Float (double-precision)") (InputAction :type "InputAction Object Reference" :default "/Game/Inputs/Player_Walk.Player_Walk"))
  (bind _returnvalue (`KismetMathLibrary.Conv_Vector2DToVector` ActionValue))
  ;[1 0.1569 0.1961] Get Walk Input
  (:`Triggered`
    (if (not (`self.bDashing`))
      ;[0.3765 0.6863 1] Move and set rotation
      (`self.AddMovementInput` _returnvalue)
      (`SceneComponent.K2_SetWorldRotation` (`self.Mesh`) (`KismetMathLibrary.MakeRotFromX` _returnvalue) false false)
      (`SceneComponent.K2_AddLocalRotation` (`self.Mesh`) (struct :`Yaw` -90.0) false false)
      (set `self.Moving` true))))

(event `EnhancedInput|/Game/Inputs/Player_Dash`
  (params (ActionValue :type Boolean) (ElapsedSeconds :type "Float (double-precision)") (TriggeredSeconds :type "Float (double-precision)") (InputAction :type "InputAction Object Reference" :default "/Game/Inputs/Player_Dash.Player_Dash"))
  (:`Triggered`
    (`|ExecutionSequence`
      (:`then_0`
        (`self.Dash` 0.2 0.75))
      (:`then_1`
        (`self.Double Dash`)))))

(event `self.CapsuleComponent.OnComponentHit`
  (params (HitComponent :type "PrimitiveComponent Object Reference") (OtherActor :type "Actor Object Reference") (OtherComp :type "PrimitiveComponent Object Reference") (NormalImpulse :type "Vector Structure") (Hit :type "HitResult Structure (by ref)"))
  ;[1 0.1569 0.1961] Hit on Capsule Component
  (if (`KismetMathLibrary.ClassIsChildOf` (`GameplayStatics.GetObjectClass` OtherActor) "/Script/Dashing_Hot.Enemy")
    (set `self.Punching` true))
  ;[0.3882 1 0.3333] Stop Dashing
  (`self.Stop Dashing`))

(event `EnhancedInput|/Game/Inputs/Pause_Game`
  (params (ActionValue :type Boolean) (ElapsedSeconds :type "Float (double-precision)") (TriggeredSeconds :type "Float (double-precision)") (InputAction :type "InputAction Object Reference" :default "/Game/Inputs/Pause_Game.Pause_Game"))
  (bind _returnvalue (`GameplayStatics.GetPlayerController` 0))
  (:`Started`
    (bind _returnvalue_2 (`|CreateWidget` "/Game/UI/Pause_Menu/Pause.Pause_C"))
    (`UserWidget.AddToViewport` _returnvalue_2 0)
    (set `PlayerController.bShowMouseCursor` true _returnvalue)
    (`WidgetBlueprintLibrary.SetInputMode_UIOnlyEx` _returnvalue null)
    (`GameplayStatics.SetGamePaused` true)))

(fn `GetAndFaceDashDirection`
  (returns (dashDirection :type "Vector Structure"))
  (bind _playercontroller (`self.PlayerController`))
  (bind (_locationx _locationy) (`PlayerController.GetMousePosition` _playercontroller))
  ;[1 1 1] Get direction vector (from player to click position)
  (bind _returnvalue (`self.GetMousePositionFromPlayer` (`PlayerController.ProjectWorldLocationToScreen` _playercontroller (`self.K2_GetActorLocation`) false) (`KismetMathLibrary.MakeVector2D` _locationx _locationy)))
  (bind _returnvalue_2 (`KismetMathLibrary.Normal` (`KismetMathLibrary.Conv_Vector2DToVector` _returnvalue)))
  ;[1 1 1] Make player face click direction
  (`SceneComponent.K2_SetWorldRotation` (`self.Mesh`) (`KismetMathLibrary.MakeRotFromX` _returnvalue_2) false false)
  (`SceneComponent.K2_AddLocalRotation` (`self.Mesh`) (struct :`Yaw` -90.0) false false)
  (return _returnvalue_2))

(fn `UserConstructionScript`)