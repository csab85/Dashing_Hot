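; Enemy VFX actor that repeatedly plays a teleport disappear and reappear effect on its skeletal mesh, starting at BeginPlay.
; The Sumir (vanish) and Aparecer (appear) timelines drive the "Boundary" parameter on dynamic EnemyShooterVFX materials in both mesh slots.
; Each phase spawns its own attached Niagara teleport system.
; Delays chained from the timeline Update pins, rather than Finished, alternate the phases in an endless loop.
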(event `self.ReceiveBeginPlay`
  (bind _skeletalmesh (`self.SkeletalMesh`))
  (bind _skeletalmesh_2 (`self.SkeletalMesh`))
  (bind _returnvalue (`PrimitiveComponent.CreateDynamicMaterialInstance` _skeletalmesh 0 "/Game/Art/Materials/Characters/Material_EnemyShooterVFX_Inst.Material_EnemyShooterVFX_Inst" "None" :!label _label))
  (bind _returnvalue_2 (`PrimitiveComponent.CreateDynamicMaterialInstance` _skeletalmesh 1 "/Game/Art/Materials/Characters/Material_EnemyShooterVFX_Inst.Material_EnemyShooterVFX_Inst" "None"))
  (`NiagaraFunctionLibrary.SpawnSystemAttached` "/Game/Art/NE_System/Enemy/NS_Teleport.NS_Teleport" _skeletalmesh "None" (0.0 0.0 0.0) (struct) "KeepRelativeOffset")
  (bind (_direction _newtrack_0) (`Timeline|Sumir` :!via `PlayFromStart`)
    (:`Update`
      (`MaterialInstanceDynamic.SetScalarParameterValue` _returnvalue "Boundary" _newtrack_0)
      (`MaterialInstanceDynamic.SetScalarParameterValue` _returnvalue_2 "Boundary" _newtrack_0)
      (`KismetSystemLibrary.Delay` 3.0)
      (bind _returnvalue_3 (`PrimitiveComponent.CreateDynamicMaterialInstance` _skeletalmesh_2 1 "/Game/Art/Materials/Characters/Material_EnemyShooterVFX_Inst.Material_EnemyShooterVFX_Inst" "None"))
      (bind _returnvalue_4 (`PrimitiveComponent.CreateDynamicMaterialInstance` _skeletalmesh_2 0 "/Game/Art/Materials/Characters/Material_EnemyShooterVFX_Inst.Material_EnemyShooterVFX_Inst" "None"))
      (`NiagaraFunctionLibrary.SpawnSystemAttached` "/Game/Art/NE_System/Enemy/NS_Teleport1.NS_Teleport1" _skeletalmesh_2 "None" (0.0 0.0 0.0) (struct) "KeepRelativeOffset")
      (bind (_direction_2 _newtrack_0_2) (`Timeline|Aparecer` :!via `PlayFromStart`)
        (:`Update`
          (`MaterialInstanceDynamic.SetScalarParameterValue` _returnvalue_3 "Boundary" _newtrack_0_2)
          (`MaterialInstanceDynamic.SetScalarParameterValue` _returnvalue_4 "Boundary" _newtrack_0_2)
          (`KismetSystemLibrary.Delay` 3.0)
          (goto _label))))))

(fn `UserConstructionScript`)